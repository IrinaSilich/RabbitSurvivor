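; Game mode that links to the game instance and opens the game-over and rabbit-collection UI.
; On BeginPlay it registers itself on BP_BaseGameInstance and triggers that instance's save game setup.
; GameOver shows W_GameOver, while RabbitsAreTaken passes the collector's row index to a new W_RabbitsCollection widget and then fires the RabbitsCollectionWidgetOpened dispatcher.
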(event `self.ReceiveBeginPlay`
  (`parent.ReceiveBeginPlay`)
  (bind _asbp_base_game_instance (cast `/Game/Blueprints/BP_BaseGameInstance` (`GameplayStatics.GetGameInstance`)))
  (set `/Game/Blueprints/BP_BaseGameInstance.GameMode` self _asbp_base_game_instance)
  (`/Game/Blueprints/BP_BaseGameInstance.SaveGameSetup` _asbp_base_game_instance))

(event `self.GameOver`
  (bind _returnvalue (`|CreateWidget` "/Game/Blueprints/UI/W_GameOver.W_GameOver_C"))
  (`UserWidget.AddToViewport` _returnvalue 0))

(event `self.RabbitsAreTaken`
  (params (CollectorRowIndex :type Integer))
  (bind _returnvalue (`|CreateWidget` "/Game/Blueprints/UI/W_RabbitsCollection.W_RabbitsCollection_C" null CollectorRowIndex))
  (`UserWidget.AddToViewport` _returnvalue 0)
  (`self.RabbitsCollectionWidgetOpened`))

(fn `UserConstructionScript`)