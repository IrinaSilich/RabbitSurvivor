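; Player controller for a rabbit-colony game that sets up the HUD, caches the living hole and handles touch commands.
; Tapping a food spot with food and a free slot has the hole spawn a collector rabbit assigned to a chosen seat.
; Tapping a frozen or sick rabbit not pending rescue stores it and spawns a rescuer; tapping any other rabbit cancels its food collection.
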(event `self.ReceiveBeginPlay`
  (bind _returnvalue (`|CreateWidget` "/Game/Blueprints/UI/W_PlayerHUD.W_PlayerHUD_C"))
  (`UserWidget.AddToViewport` _returnvalue 0)
  (bind _returnvalue_2 (`GameplayStatics.GetActorOfClass` "/Game/Blueprints/BP_LivingHole.BP_LivingHole_C"))
  (set `self.LivingHole` _returnvalue_2)
  (`WidgetBlueprintLibrary.SetInputMode_GameAndUIEx` self null)
  (set `self.bShowMouseCursor` true))

(event `InputTouch`
  (params (Location :type "Vector Structure") (FingerIndex :type "ETouchIndex Enum"))
  (bind _hitresult (`self.GetHitResultUnderFingerByChannel` "Touch1" "TraceTypeQuery1"))
  (bind _livinghole (`self.LivingHole`))
  (bind _livinghole_2 (`self.LivingHole`))
  (:`Pressed`
    ;[1 1 1] Разные виджеты вызываются в зависимости от того, по какому месту было нажатие
    (bind _asbp_food_spot (cast `/Game/Blueprints/BP_FoodSpot` (`.HitActor` (`GameplayStatics.BreakHitResult` _hitresult)))
      (:`then`
        (if (and (> (`FoodSpot.GetCurrentFood` _asbp_food_spot) 0.0) (not (>= (`KismetArrayLibrary.Array_Length` (`FoodSpot.GetRabbitsAssigned` _asbp_food_spot)) (`FoodSpot.MaxRabbitsAssignedToBush` _asbp_food_spot))))
          (bind _returnvalue (`FoodSpot.ChooseCollectionSeat` _asbp_food_spot))
          (`/Engine/EditorBlueprintResources/StandardMacros.IsValid` _livinghole
            (:`Is Valid`
              (bind _returnvalue_2 (`LivingHole.SpawnRabbit` _livinghole "CollectFood" _asbp_food_spot _returnvalue)))
            (:`Is Not Valid`
              _))
          (`FoodSpot.IncreaseRabbitsAssigned` _asbp_food_spot _returnvalue_2)
          (`FoodSpot.SetRabbitFreezingRate` _asbp_food_spot)))
      (:`CastFailed`
        (bind _asbp_rabbit (cast `/Game/Blueprints/BP_Rabbit` (`.HitActor` (`GameplayStatics.BreakHitResult` _hitresult))))
        (bind ((`IsFrozen` _isfrozen) (`IsSick` _issick) (`IsPendingRescue` _ispendingrescue)) (break `RabbitParameters` (`Rabbit.GetRabbitParameters` _asbp_rabbit)))
        (if (or _isfrozen _issick)
          (if (not _ispendingrescue)
            (set `self.FrozenRabbit` _asbp_rabbit)
            (`/Engine/EditorBlueprintResources/StandardMacros.IsValid` _livinghole_2
              (:`Is Valid`
                (`LivingHole.SpawnRabbit` _livinghole_2 "Rescue" null null))))
          (else
            (`Rabbit.CancelFoodCollection` _asbp_rabbit)))))))

(fn `UserConstructionScript`)