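; Behavior tree task in which a rabbit gathers food from its assigned food spot.
; It turns the rabbit to match its collection seat, sets a task-processing flag for animation, and starts a looping timer.
; Each tick moves food from the spot into the rabbit's resources until it is full or the spot is empty.
; It then succeeds, clearing the rabbit's assignment if the spot is depleted; failed initial checks fail the task.
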(event `self.ReceiveExecute`
  (params (OwnerActor :type "Actor Object Reference"))
  (bind _rabbit (`self.Rabbit`))
  (bind (_rabbitresources_currentamount _rabbitresources_increaseamount _rabbitresources_maxamount _rabbitresources_timeforcollecting) (break `RabbitResourceCollection` (`Rabbit.RabbitResources` (`self.Rabbit`))))
  (bind (_rabbitparameters_currentclass _rabbitparameters_taskassigned _rabbitparameters_warmthstamina _rabbitparameters_istaskprocessed) (break `RabbitParameters` (`Rabbit.RabbitParameters` (`self.Rabbit`))))
  (bind _ascontroller (cast `Controller` OwnerActor)
    (:`then`
      (bind _asbp_rabbit (cast `/Game/Blueprints/BP_Rabbit` (`Controller.K2_GetPawn` _ascontroller))
        (:`then`
          (set `self.Rabbit` _asbp_rabbit)
          (if (> _rabbitresources_timeforcollecting 0.0)
            (if (> (`FoodSpot.GetCurrentFood` (`.AssignedFoodSpot` (break `RabbitParameters` (`Rabbit.RabbitParameters` (`self.Rabbit`))))) 0.0)
              ;[1 1 1] Кролик начал выполнять задачу (используется для анимаций)
              (`|VariableSetRef` _rabbitparameters_istaskprocessed true)
              ;[1 1 1] Когда кролик подсаживается к кусту, он поворачивается в сторону того collection seat, в которое назначен
              (`Actor.K2_SetActorRotation` _rabbit (`SceneComponent.K2_GetComponentRotation` (`.AssignedCollectionSeat` (break `RabbitParameters` (`Rabbit.RabbitParameters` _rabbit)))) false)
              (bind _returnvalue (`KismetSystemLibrary.K2_SetTimerDelegate` (delegate `CustomEvent`) _rabbitresources_timeforcollecting true))
              (set `self.CollectionTimer` _returnvalue)
              (else
                (`self.FinishExecute` false)))
            (else
              (`self.FinishExecute` false))))
        (:`CastFailed`
          (`self.FinishExecute` false))))
    (:`CastFailed`
      (`self.FinishExecute` false))))

(event `CustomEvent`
  (bind _rabbit (`self.Rabbit`))
  (bind (_rabbitresources_currentamount _rabbitresources_increaseamount _rabbitresources_maxamount _rabbitresources_timeforcollecting) (break `RabbitResourceCollection` (`Rabbit.RabbitResources` (`self.Rabbit`))))
  (bind (_rabbitparameters_currentclass _rabbitparameters_taskassigned _rabbitparameters_warmthstamina _rabbitparameters_istaskprocessed) (break `RabbitParameters` (`Rabbit.RabbitParameters` (`self.Rabbit`))))
  (bind ((`TaskAssigned` _taskassigned) (`AssignedFoodSpot` _assignedfoodspot)) (break `RabbitParameters` (`Rabbit.RabbitParameters` _rabbit)))
  (bind ((`IsFrozen` _isfrozen) (`AssignedFoodSpot` _assignedfoodspot_2)) (break `RabbitParameters` (`Rabbit.RabbitParameters` (`self.Rabbit`))))
  (if (`KismetMathLibrary.NearlyEqual_FloatFloat` _rabbitresources_currentamount _rabbitresources_maxamount)
    (`KismetSystemLibrary.K2_ClearAndInvalidateTimerHandle` (`self.CollectionTimer`) :!label _label)
    (if (not (> (`FoodSpot.GetCurrentFood` (`.AssignedFoodSpot` (break `RabbitParameters` (`Rabbit.RabbitParameters` (`self.Rabbit`))))) 0.0))
      (`|VariableSetRef` _taskassigned)
      (`KismetArrayLibrary.Array_RemoveItem` (`FoodSpot.GetRabbitsAssigned` _assignedfoodspot) _rabbit))
    ;[1 1 1] Кролик закончил выполнять задачу (используется для анимаций)
    (`|VariableSetRef` _rabbitparameters_istaskprocessed)
    (`self.FinishExecute` true)
    (elif (> (`FoodSpot.GetCurrentFood` _assignedfoodspot_2) 0.0)
      (`FoodSpot.SetCurrentFood` _assignedfoodspot_2 (- (`FoodSpot.GetCurrentFood` _assignedfoodspot_2) _rabbitresources_increaseamount))
      (set `Rabbit.RabbitResources` (make `RabbitResourceCollection` (+ _rabbitresources_currentamount _rabbitresources_increaseamount) _rabbitresources_increaseamount _rabbitresources_maxamount _rabbitresources_timeforcollecting) (`self.Rabbit`))
      (else
        (goto _label)))))