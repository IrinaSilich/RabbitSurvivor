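; BP_Rabbit is a rabbit with warmth and food collection progress widgets attached.
; On BeginPlay it runs the parent logic and passes itself to both widgets as their rabbit reference.
; A looping timer polls the task state in RabbitParameters and shows the food progress bar only during task processing, hiding it while the rabbit runs between burrows.
; The construction script assigns a random skeletal mesh from RabbitSkins.
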(event `self.ReceiveBeginPlay`
  (`parent.ReceiveBeginPlay`)
  ;[1 1 1] Устанавливаем ссылки на кролика в виджетах
  (bind _asw_warmth_bar (cast `/Game/Blueprints/UI/W_WarmthBar` (`WidgetComponent.GetWidget` (`self.W_WarmthBar`)))
    (:`then`
      (set `/Game/Blueprints/UI/W_WarmthBar.Rabbit` self _asw_warmth_bar))
    (:`CastFailed`
      _))
  (bind _asw_food_collection_progress (cast `/Game/Blueprints/UI/W_FoodCollectionProgress` (`WidgetComponent.GetWidget` (`self.W_FoodCollectionProgressBar`))))
  (set `/Game/Blueprints/UI/W_FoodCollectionProgress.Rabbit` self _asw_food_collection_progress)
  ;[1 1 1] Скрываем прогресс бар сбора еды, пока кролик бегает от норы к норе
  (`KismetSystemLibrary.K2_SetTimerDelegate` (delegate `CustomEvent`) 0.1 true))

(event `CustomEvent`
  (bind _w_foodcollectionprogressbar (`self.W_FoodCollectionProgressBar`))
  ;[1 1 1] Скрываем прогресс бар сбора еды, пока кролик бегает от норы к норе
  (if (`.IsTaskProcessed` (break `RabbitParameters` (`self.RabbitParameters`)))
    (`SceneComponent.SetVisibility` _w_foodcollectionprogressbar true false)
    (else
      (`SceneComponent.SetVisibility` _w_foodcollectionprogressbar false false))))

(fn `UserConstructionScript`
  (bind _rabbitskins (`self.RabbitSkins`))
  ;[1 1 1] Рандомные меши для кроликов
  (`SkeletalMeshComponent.SetSkeletalMeshAsset` (`self.Mesh`) (`|GetArrayItem` _rabbitskins (`KismetMathLibrary.RandomIntegerInRange` 0 (- (`KismetArrayLibrary.Array_Length` _rabbitskins) 1)))))