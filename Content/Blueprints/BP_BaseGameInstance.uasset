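; Base game instance that caches the living hole actor on init and handles saving and loading of the rabbit colony.
; SaveGameSetup loads an existing slot and triggers a frozen-rabbit check, or initializes the hole and saves, then starts a looping autosave timer.
; Saves store food, rabbit count, and regular and warming-up rabbit parameters.
; Rabbits outside the hole are appended to the saved rabbit list so they persist.
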(event `self.ReceiveInit`
  (`parent.ReceiveInit`)
  (bind _returnvalue (`GameplayStatics.GetActorOfClass` "/Game/Blueprints/BP_LivingHole.BP_LivingHole_C"))
  (set `self.LivingHole` _returnvalue))

(fn `AddRabbitsOutsideHoleParameters`
  (locals (RabbitParametersLocal :type "RabbitParameters Structure"))
  (bind _livinghole (`self.LivingHole`))
  (bind _savegamefile (`self.SaveGameFile`))
  (set `SaveGameFile.SavedRabbitsParameters` (`LivingHole.GetRabbitsParameters` _livinghole) _savegamefile)
  (set `SaveGameFile.SavedWarmingUpRabbitsParameters` (`LivingHole.GetWarmedUpRabbitsParameters` _livinghole) _savegamefile)
  (for _array_element (`LivingHole.GetRabbitsOutsideHole` (`self.LivingHole`))
    (`/Engine/EditorBlueprintResources/StandardMacros.IsValid` _array_element
      (:`Is Valid`
        (bind (_currentclass _taskassigned _warmthstamina _istaskprocessed _isfrozen) (break `RabbitParameters` (`Rabbit.GetRabbitParameters` _array_element)))
        (bind _output_get (set `local.RabbitParametersLocal` (make `RabbitParameters` _currentclass "None" _warmthstamina false _isfrozen)))
        (`KismetArrayLibrary.Array_Add` (`SaveGameFile.SavedRabbitsParameters` _savegamefile) _output_get))))
  (return))

(fn `LoadGame`
  (bind _livinghole (`self.LivingHole`))
  (bind _returnvalue (`GameplayStatics.LoadGameFromSlot` (`self.SaveSlot`)))
  (bind _asbp_save_game_file (cast `/Game/Blueprints/BP_SaveGameFile` _returnvalue))
  (`/Engine/EditorBlueprintResources/StandardMacros.IsValid` (`self.LivingHole`)
    (:`Is Valid`
      (`/Engine/EditorBlueprintResources/StandardMacros.IsValid` (`self.GameMode`)
        (:`Is Valid`
          (`LivingHole.SetRabbitsParameters` _livinghole (`SaveGameFile.SavedRabbitsParameters` _asbp_save_game_file))
          (`LivingHole.SetWarmingUpRabbitsParameters` _livinghole (`SaveGameFile.SavedWarmingUpRabbitsParameters` _asbp_save_game_file))
          (set `BaseHole.FoodAmountCollected` (`SaveGameFile.SavedFoodAmountCollected` _asbp_save_game_file) (`self.LivingHole`))
          (set `BaseHole.TotalRabbitsCount` (`SaveGameFile.SavedTotalRabbitsCount` _asbp_save_game_file) (`self.LivingHole`)))))))

(fn `SaveGame`
  (bind _livinghole (`self.LivingHole`))
  (bind _savegamefile (`self.SaveGameFile`))
  (`/Engine/EditorBlueprintResources/StandardMacros.IsValid` (`self.SaveGameFile`)
    (:`Is Valid`
      (`/Engine/EditorBlueprintResources/StandardMacros.IsValid` (`self.LivingHole`)
        (:`Is Valid`
          (`/Engine/EditorBlueprintResources/StandardMacros.IsValid` (`self.GameMode`)
            (:`Is Valid`
              ;[1 1 1] Учитываем данные кроликов, которые на момент сохранения игры находились вне норы
              (`self.AddRabbitsOutsideHoleParameters`)
              (set `SaveGameFile.SavedFoodAmountCollected` (`BaseHole.FoodAmountCollected` _livinghole) _savegamefile)
              (set `SaveGameFile.SavedTotalRabbitsCount` (`BaseHole.TotalRabbitsCount` _livinghole) _savegamefile)
              (`GameplayStatics.SaveGameToSlot` (`self.SaveGameFile`) (`self.SaveSlot`)))))))))

(fn `SaveGameSetup`
  (bind _livinghole (`self.LivingHole`))
  (bind _returnvalue (`GameplayStatics.CreateSaveGameObject` "/Game/Blueprints/BP_SaveGameFile.BP_SaveGameFile_C"))
  (set `self.SaveGameFile` _returnvalue)
  (bind _returnvalue_2 (`GameplayStatics.DoesSaveGameExist` (`self.SaveSlot`)))
  (if _returnvalue_2
    (`self.LoadGame`)
    (`LivingHole.CheckForFrozenRabbitsInGeneralSection` (`self.LivingHole`))
    (else
      (`/Engine/EditorBlueprintResources/StandardMacros.IsValid` _livinghole
        (:`Is Valid`
          (`LivingHole.InitHole` _livinghole))
        (:`Is Not Valid`
          _))
      (`self.SaveGame`)))
  (bind _returnvalue_3 (`KismetSystemLibrary.K2_SetTimer` null "SaveGame" (`self.SaveGameInterval`) true))
  (set `self.SaveGameTimer` _returnvalue_3))